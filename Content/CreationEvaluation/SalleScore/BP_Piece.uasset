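; BP_Piece is a collectible coin that adds to the score of the Salle4 room when the player picks it up.
; Box overlap by BP_ThirdPersonCharacter plays the Dispear timeline, which spins the Cylinder on its roll axis by TurnSpeed times Speed each update.
; When the timeline finishes, it destroys the actor and calls AddScore on the character's Salle reference, cast to Salle4.
; Tick stores DeltaSeconds, but the spin does not use it.
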(event OnComponentBeginOverlap(Box)
  (params (OverlappedComponent :type Primitive%20Component%20Object%20Reference) (OtherActor :type Actor%20Object%20Reference) (OtherComp :type Primitive%20Component%20Object%20Reference) (OtherBodyIndex :type Integer) (bFromSweep :type Boolean) (SweepResult :type Hit%20Result%20Structure%20%28by%20ref%29))
  (bind _cylinder (Variables|Default|GetCylinder))
  (bind _returnvalue (Transformation|GetWorldRotation _cylinder))
  (bind _asbp_third_person_character (Utilities|Casting|CastToBP_ThirdPersonCharacter OtherActor))
  (bind _turnspeed (Timeline|Dispear Play)
    (:Update
      (Transformation|SetWorldRotation _cylinder (Math|Rotator|MakeRotator (+ (* _turnspeed (Variables|Default|GetSpeed)) (.roll _returnvalue)) (.pitch _returnvalue) (.yaw _returnvalue)) false false))
    (:Finished
      (Actor|DestroyActor)
      (bind _assalle_4 (Utilities|Casting|CastToSalle4 (Variables|/Game/ThirdPerson/Blueprints/BP_ThirdPersonCharacter.BP_ThirdPersonCharacter_C|GetSalle _asbp_third_person_character)))
      (Default|AddScore _assalle_4))))

(event EventBeginPlay)

(event Collision|EventActorBeginOverlap
  (params (OtherActor :type Actor%20Object%20Reference)))

(event EventTick
  (params (DeltaSeconds :type Float%20%28single-precision%29))
  (Variables|Default|Setdelta DeltaSeconds))

(fn ConstructionScript)