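; BP_IA is an AI-controlled enemy that can track the player or return to where it started.
; It caches its starting location as BaseLocation on BeginPlay.
; TrackPlayer and Replace cast its AI controller to BP_EnemyController and delegate to it, either to track the player or to move back to BaseLocation.
; Nothing in this Blueprint calls either function.
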(event EventBeginPlay
  (Variables|Default|SetbaseLocation (Transformation|GetActorLocation)))

(fn ConstructionScript)

(fn TrackPlayer
  (bind _asbp_enemy_controller (Utilities|Casting|CastToBP_EnemyController (AI|GetAIController self)))
  (Default|TrackPlayer _asbp_enemy_controller))

(fn Replace
  (bind _asbp_enemy_controller (Utilities|Casting|CastToBP_EnemyController (AI|GetAIController self)))
  (Default|MoveTO _asbp_enemy_controller (Variables|Default|GetbaseLocation)))